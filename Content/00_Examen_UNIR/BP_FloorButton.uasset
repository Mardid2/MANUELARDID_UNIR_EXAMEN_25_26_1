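; Floor button actor that opens and closes a linked Door while the first-person character stands in its trigger box.
; Box overlaps set an inside flag and enable or disable the actor's input for player controller 0.
; Pressing E toggles the button: activation opens the Door and lights the hieroglyph material only if enough keys are collected, and deactivation closes it and turns the glow off.
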(event `Key|E`
  (params (Key :type "Key Structure"))
  (bind _door (`self.Door`))
  ; Input
  (:`Pressed`
    (if (`self.PlayerIsInside`)
      (bind _output_get (set `self.ButtonActivated` (not (`self.ButtonActivated`))))
      (if _output_get
        (if (>= (`/Game/00_Examen_UNIR/BP_Door.KeysCollected` _door) (`/Game/00_Examen_UNIR/BP_Door.RequiredKeys` _door))
          (`PrimitiveComponent.SetMaterial` (`self.SM_hieroglyph_007`) 0 "/Game/00_Examen_UNIR/M_Emission_ON.M_Emission_ON")
          (`/Game/00_Examen_UNIR/BP_Door.Open` (`self.Door`) true))
        (else
          (`PrimitiveComponent.SetMaterial` (`self.SM_hieroglyph_007`) 0 "/Game/00_Examen_UNIR/M_Emission_OFF.M_Emission_OFF")
          (`/Game/00_Examen_UNIR/BP_Door.Open` (`self.Door`) false))))))

(event `self.Box.OnComponentBeginOverlap`
  (params (OverlappedComponent :type "PrimitiveComponent Object Reference") (OtherActor :type "Actor Object Reference") (OtherComp :type "PrimitiveComponent Object Reference") (OtherBodyIndex :type Integer) (bFromSweep :type Boolean) (SweepResult :type "HitResult Structure (by ref)"))
  ; Detect player inside
  (cast `/Game/FirstPerson/Blueprints/BP_FirstPersonCharacter` OtherActor)
  (set `self.PlayerIsInside` true)
  (`self.EnableInput` (`GameplayStatics.GetPlayerController` 0)))

(event `self.Box.OnComponentEndOverlap`
  (params (OverlappedComponent :type "PrimitiveComponent Object Reference") (OtherActor :type "Actor Object Reference") (OtherComp :type "PrimitiveComponent Object Reference") (OtherBodyIndex :type Integer))
  ; Detect player inside
  (cast `/Game/FirstPerson/Blueprints/BP_FirstPersonCharacter` OtherActor)
  (set `self.PlayerIsInside` false)
  (`self.DisableInput` (`GameplayStatics.GetPlayerController` 0)))

(fn `UserConstructionScript`)