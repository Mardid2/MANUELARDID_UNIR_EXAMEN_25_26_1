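; BP_DOOR is a double sliding door that opens only after enough keys have been collected.
; It counts keys through OnKeyCollected, printing the tally on screen.
; When the count meets RequiredKeys, Open plays or reverses a Timeline that lerps both panels apart along local X from positions cached at BeginPlay.
; Otherwise, it prints the required key count in Spanish.
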(event `self.ReceiveBeginPlay`
  ; Init
  (set `self.InitPos_RightDoor` (`SceneComponent.RelativeLocation` (`self.RightDoor`)))
  (set `self.InitPos_LeftDoor` (`SceneComponent.RelativeLocation` (`self.LeftDoor`))))

(event `Open`
  (params (Open :type Boolean))
  (bind _initpos_rightdoor (`self.InitPos_RightDoor`))
  (bind _initpos_leftdoor (`self.InitPos_LeftDoor`))
  ; Open Logic
  (if (>= (`self.KeysCollected`) (`self.RequiredKeys`))
    (if Open
      (bind (_direction _newtrack_0) (`Timeline|Timeline` :!label _label)
        (:`Update`
          (`SceneComponent.K2_SetRelativeLocation` (`self.RightDoor`) (`KismetMathLibrary.VLerp` _initpos_rightdoor (+ _initpos_rightdoor (80.0 0.0 0.0)) _newtrack_0) false false)
          (`SceneComponent.K2_SetRelativeLocation` (`self.LeftDoor`) (`KismetMathLibrary.VLerp` _initpos_leftdoor (+ _initpos_leftdoor (-80.0 0.0 0.0)) _newtrack_0) false false)))
      (else
        (goto _label :!via `Reverse`)))
    (else
      (`KismetSystemLibrary.PrintString` (`KismetStringLibrary.Concat_StrStr` "Llaves necesarias para abrir la puerta: " (`KismetStringLibrary.Conv_IntToString` (`self.RequiredKeys`)))))))

(event `OnKeyCollected`
  ; Key Collection
  (bind _output_get (set `self.KeysCollected` (+ (`self.KeysCollected`) 1)))
  (`KismetSystemLibrary.PrintString` (`KismetStringLibrary.Concat_StrStr` "Llaves: " (`KismetStringLibrary.GetSubstring` (`KismetStringLibrary.Conv_IntToString` _output_get)))))

(fn `UserConstructionScript`)